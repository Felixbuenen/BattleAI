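; Command manager that turns right-mouse press, drag and release into control of a Frame for the active formations.
; Mouse down records the screen position and initializes the Frame at the cursor's world hit.
; Tick waits until screen movement exceeds the drag threshold, then updates the Frame with complex cursor traces while the button is held.
; Mouse up stops the Frame but leaves the dragging flag set.
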(event `self.HandleRightMouseDown`
  (bind (_locationx _locationy) (`PlayerController.GetMousePosition` (`GameplayStatics.GetPlayerController` 0)))
  (bind (_bblockinghit _binitialoverlap _time _distance _location) (`GameplayStatics.BreakHitResult` (`PlayerController.GetHitResultUnderCursorByChannel` (`GameplayStatics.GetPlayerController` 0) "TraceTypeQuery4" true)))
  (set `self.StartScreenPos` (`KismetMathLibrary.MakeVector2D` _locationx _locationy))
  (set `self.RightClickDown` true)
  (`FormationFrame.Init` (`self.frame`) _location _location (`self.activeFormations`)))

(event `self.HandleRightMouseUp`
  (set `self.RightClickDown` false)
  (`FormationFrame.Stop` (`self.frame`)))

(event `self.ReceiveTick`
  (params (DeltaSeconds :type "Float (single-precision)"))
  (bind (_locationx _locationy) (`PlayerController.GetMousePosition` (`GameplayStatics.GetPlayerController` 0)))
  (if (`self.RightClickDown`)
    (if (`self.IsRightClickDragging`)
      (`FormationFrame.Update` (`self.frame`) (`.Location` (`GameplayStatics.BreakHitResult` (`PlayerController.GetHitResultUnderCursorByChannel` (`GameplayStatics.GetPlayerController` 0) "TraceTypeQuery4" true))) :!label _label)
      (elif (> (`KismetMathLibrary.VSize2D` (- (`self.StartScreenPos`) (`KismetMathLibrary.MakeVector2D` _locationx _locationy))) (`self.DragThreshold`))
        (set `self.IsRightClickDragging` true)
        (goto _label)))))

(fn `UserConstructionScript`)