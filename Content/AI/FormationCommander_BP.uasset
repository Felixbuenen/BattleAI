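; Formation commander character that leads a group of soldiers to a destination.
; GoToLocation stores and sets up the final destination, then starts movement along the supplied path.
; While moving, each tick passes the commander's transform, destination and walk speed to every soldier's FollowCommander.
; The largest returned distance drives the commander's speed on the next tick, slowing it as soldiers fall behind.
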(event `self.ReceiveBeginPlay`)

(event `self.ReceiveTick`
  (params (DeltaSeconds :type "Float (single-precision)"))
  (bind _capsulecomponent (`self.CapsuleComponent`))
  (bind (_x _y _z) (`KismetMathLibrary.BreakRotIntoAxes` (`SceneComponent.K2_GetComponentRotation` _capsulecomponent)))
  (if (`self.isMoving`)
    (`|ExecutionSequence`
      (:`then_0`
        (bind _output_get (set `CharacterMovementComponent.MaxWalkSpeed` (`KismetMathLibrary.MapRangeClamped` (`self.MaxSoldierDist`) 50.0 300.0 (`self.MaxSpeed`) (`self.MinSpeed`)) (`self.CharacterMovement`))))
      (:`then_1`
        (set `self.MaxSoldierDist` 0.0)
        (for _array_element (`self.Soldiers`)
          (bind _assoldier_bp (cast `/Game/Blueprints/Soldier_BP` _array_element))
          (bind _disttogoal (`/Game/Blueprints/Soldier_BP.FollowCommander` _assoldier_bp (`SceneComponent.K2_GetComponentLocation` _capsulecomponent) (`SceneComponent.GetForwardVector` _capsulecomponent) (`self.FinalDest`) (`KismetMathLibrary.MakeRotationFromAxes` _x _y _z) (`CharacterMovementComponent.MaxWalkSpeed` (`self.CharacterMovement`))))
          (if (> _disttogoal (`self.MaxSoldierDist`))
            (set `self.MaxSoldierDist` _disttogoal)))))))

(fn `GoToLocation`
  (params (Location :type "Vector Structure") (Path :type "GlobalPath Object Reference"))
  (`self.SetupFinalDestination` Location)
  (set `self.FinalDest` Location)
  (`self.MoveToLocation` Path))

(fn `UserConstructionScript`)