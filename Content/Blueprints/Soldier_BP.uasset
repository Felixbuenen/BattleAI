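; Soldier character that holds an offset slot in a formation around a commander and has a sphere collider for clicks.
; FollowCommander scales walk speed by distance to a look-ahead slot point, re-paths there on a throttled timer and returns its distance from the slot.
; GotoFinalLocationandOrientation moves it to its final slot, then Tick interpolates rotation to the commander's orientation at a speed derived from the yaw difference.
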(event `self.ReceiveBeginPlay`
  (`PrimitiveComponent.SetCollisionProfileName` (`self.Sphere`) "SoldierClickCollider"))

(event `self.ReceiveTick`
  (params (DeltaSeconds :type "Float (single-precision)"))
  (if (`self.UpdateRotation`)
    (`self.SetCorrectOrientation` DeltaSeconds)
    (set `self.UpdateRotation` (!= (`self.K2_GetActorRotation`) (`self.GoalRotation`) :`ErrorTolerance` 0.01))))

(event `self.GoToFinalLocationAndOrientation`
  (params (commLocation :type "Vector Structure") (commOrientation :type "Rotator Structure"))
  (bind (_x _y) (`KismetMathLibrary.GetAxes` commOrientation))
  (`AITask_MoveTo.AIMoveTo` (`AIBlueprintHelperLibrary.GetAIController` self) (`KismetMathLibrary.MakeVector` (.x (+ commLocation (+ (* _x (.x (`self.MyOffset`))) (* _y (.y (`self.MyOffset`)))))) (.y (+ commLocation (+ (* _x (.x (`self.MyOffset`))) (* _y (.y (`self.MyOffset`))))))) null -1.0 "Disable"
    (:`OnMoveFinished`
      (`|ExecutionSequence`
        (:`then_0`
          (bind _output_get (set `self.GoalRotation` commOrientation)))
        (:`then_1`
          (bind _output_get_2 (set `self.RotationDelta` (`KismetMathLibrary.Abs` (- (.yaw _output_get) (.yaw (`self.K2_GetActorRotation`))))))
          (if (> _output_get_2 180.0)
            (bind _output_get_3 (set `self.RotationDelta` (- _output_get_2 180.0)))
            (set `self.UpdateRotationLerpSpeed` (/ 1.0 (/ _output_get_3 (* 180.0 (`self.UpdateRotationSpeed`)))))
            (else
              (set `self.UpdateRotationLerpSpeed` (/ 1.0 (/ (`self.RotationDelta`) (* 180.0 (`self.UpdateRotationSpeed`))))))))
        (:`then_2`
          (set `self.UpdateRotation` true))))))

(fn `FollowCommander`
  (params (CommanderPosition :type "Vector Structure") (CommanderForward :type "Vector Structure") (FinalDestination :type "Vector Structure") (CommanderOrientation :type "Rotator Structure") (MaxSpeed :type "Float (double-precision)"))
  (returns (DistToGoal :type "Float (double-precision)"))
  (bind _returnvalue (`KismetMathLibrary.GreaterGreater_VectorRotator` (`self.MyOffset`) CommanderOrientation))
  (bind _returnvalue_2 (`SceneComponent.K2_GetComponentLocation` (`self.CapsuleComponent`)))
  (bind _returnvalue_3 (+ _returnvalue CommanderPosition))
  (bind _returnvalue_4 (`KismetMathLibrary.VSize` (- _returnvalue_3 _returnvalue_2)))
  (bind _returnvalue_5 (+ _returnvalue_3 (* CommanderForward (`KismetMathLibrary.FMin` (`KismetMathLibrary.VSize` (- (+ _returnvalue FinalDestination) _returnvalue_2)) (* MaxSpeed 2.0)))))
  (set `CharacterMovementComponent.MaxWalkSpeed` (`KismetMathLibrary.MapRangeClamped` (`KismetMathLibrary.VSize` (- _returnvalue_2 _returnvalue_5)) 20.0 300.0 10.0 200.0) (`self.CharacterMovement`))
  (bind _output_get (set `self.FindLocationInterval` (- (`self.FindLocationInterval`) (`GameplayStatics.GetWorldDeltaSeconds`))))
  (if (<= _output_get 0.0)
    (set `self.FindLocationInterval` 0.5)
    (`AIController.MoveToLocation` (`AIBlueprintHelperLibrary.GetAIController` self) _returnvalue_5 0.01 true true false true null true)
    (return _returnvalue_4)
    (else
      (return _returnvalue_4))))

(fn `SetCorrectOrientation`
  (params (`delta time` :type "Float (double-precision)"))
  (`self.K2_SetActorRotation` (`KismetMathLibrary.RInterpTo` (`self.K2_GetActorRotation`) (`self.GoalRotation`) `delta time` (`self.UpdateRotationLerpSpeed`))))

(fn `UserConstructionScript`)