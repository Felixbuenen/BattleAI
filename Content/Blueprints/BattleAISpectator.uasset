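; BattleAISpectator is a free-flying spectator pawn, steered by movement and rotation input relative to the control rotation.
; Tick consumes the movement input and eases an offset toward its normalized direction, or more quickly back to zero when idle.
; The offset moves the actor without sweep, scaled by move speed but not by delta time, and holding FastMove doubles it.
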(event `InputAxis|MoveForward`
  (params (AxisValue :type "Float (single-precision)"))
  (`self.AddMovementInput` (`KismetMathLibrary.GetForwardVector` (`self.GetControlRotation`)) AxisValue))

(event `InputAxis|MoveUp`
  (params (AxisValue :type "Float (single-precision)"))
  (`self.AddMovementInput` (`KismetMathLibrary.GetUpVector` (`self.GetControlRotation`)) AxisValue))

(event `InputAxis|MoveRight`
  (params (AxisValue :type "Float (single-precision)"))
  (`self.AddMovementInput` (`KismetMathLibrary.GetRightVector` (`self.GetControlRotation`)) AxisValue))

(event `InputAxis|RotateX`
  (params (AxisValue :type "Float (single-precision)"))
  (`self.AddControllerYawInput` AxisValue))

(event `InputAxis|RotateY`
  (params (AxisValue :type "Float (single-precision)"))
  (`self.AddControllerPitchInput` AxisValue))

(event `self.ReceiveTick`
  (params (DeltaSeconds :type "Float (single-precision)"))
  (bind _returnvalue (`self.ConsumeMovementInputVector`))
  (if (< (`KismetMathLibrary.VSizeSquared` _returnvalue) 0.01)
    (bind _output_get (set `self.CurrentMoveOffset` (`KismetMathLibrary.VInterpTo` (`self.CurrentMoveOffset`) (0.0 0.0 0.0) DeltaSeconds 15.0)))
    (`self.K2_AddActorWorldOffset` (* _output_get (* (`self.MoveSpeed`) (`self.SpeedIncreaser`))))
    (else
      (bind _output_get_2 (set `self.CurrentMoveOffset` (`KismetMathLibrary.VInterpTo` (`self.CurrentMoveOffset`) (`KismetMathLibrary.Normal` _returnvalue) DeltaSeconds 5.0)))
      (`self.K2_AddActorWorldOffset` (* _output_get_2 (* (`self.MoveSpeed`) (`self.SpeedIncreaser`)))))))

(event `InputAction|FastMove`
  (params (Key :type "Key Structure"))
  (:`Pressed`
    (set `self.SpeedIncreaser` 2.0))
  (:`Released`
    (set `self.SpeedIncreaser` 1.0)))

(fn `UserConstructionScript`)